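; GA_Heal is a Gameplay Ability that heals the activating Hermes player character's team.
; On activation it casts the avatar to HermesPlayerCharacter, loops over GetTeamCharacters, and applies GE_Heal to each through actor target data, printing a debug message.
; EndAbility is called inside the loop body after each application, with no CommitAbility and no end call when the cast fails or the team is empty.
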(event Ability|EventActivateAbility
  (bind _returnvalue (Ability|GetAvatarActorfromActorInfo))
  (Development|PrintString "GA_Heal")
  (bind _ashermes_player_character (Utilities|Casting|CastToHermesPlayerCharacter _returnvalue))
  (for _array_element (Class|HermesPlayerCharacter|GetTeamCharacters _ashermes_player_character)
    (GameplayEffects|ApplyGameplayEffectToTarget (Ability|TargetData|AbilityTargetDatafromActor _array_element) "/Game/GE/GE_Heal.GE_Heal_C" 1 1)
    (Development|PrintString (Utilities|String|Append "Heal" (Utilities|GetObjectName _returnvalue) "to" (Utilities|GetObjectName _array_element)) true true "(R=0.000000,G=1.000000,B=0.225520,A=1.000000)")
    (Ability|EndAbility)))

(event Ability|EventOnEndAbility
  (params (bWasCancelled :type Boolean)))