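; Gameplay ability that keeps refreshing a path from the Hermes player character to a goal location.
; On activation it repeats every second, setting the goal from each BP_CPathWorldLocationDummy in the level.
; Each BP_CPathVolume then runs an async, smoothed CPath search, and successful results are converted and passed to UpdatePath.
; A nav mesh sync path call is left unconnected.
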(event Ability|EventActivateAbility
  (|RepeatAction 1.0 2100000000
    (:OnPerformAction
      (bind _ashermes_player_character (Utilities|Casting|CastToHermesPlayerCharacter (Ability|GetAvatarActorfromActorInfo)))
      (bind _outactors (Actor|GetAllActorsOfClass "/CPathfinding/Blueprints/ExampleLevelsBlueprints/BP_CPathWorldLocationDummy.BP_CPathWorldLocationDummy_C"))
      (for _array_element _outactors
        (Class|GAPathfinding|SetGoal (Transformation|GetActorLocation _array_element))
        (bind _outactors_2 (Actor|GetAllActorsOfClass "/CPathfinding/Blueprints/BP_CPathVolume.BP_CPathVolume_C"))
        (for _array_element_2 _outactors_2
          (bind _path (|FindPathAsync _array_element_2 (Transformation|GetActorLocation _ashermes_player_character) (Variables|Default|GetGoalLocation) 10 0 0.2)
            (:Success
              (bind _returnvalue (Class|GAPathfinding|ConvertCPathNode _path))
              (Class|GAPathfinding|UpdatePath _returnvalue))))))))

(event Ability|EventOnEndAbility
  (params (bWasCancelled :type Boolean)))