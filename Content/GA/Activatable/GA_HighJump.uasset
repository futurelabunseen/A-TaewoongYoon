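; GA_HighJump is a Gameplay Ability that makes the Hermes player character perform a boosted jump.
; On activation it prints a debug string, saves the character's JumpZVelocity, swaps in HighJumpVelocity, calls Jump and assigns a landed delegate.
; Landing restores the saved velocity and ends the ability; OnEndAbility is empty, so that callback is the only place the restore happens.
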(event Custom|LandedDelegate_이벤트
  (params (Hit :type Hit%20Result%20Structure%20%28by%20ref%29))
  (Variables|/Script/Engine.CharacterMovementComponent|SetJumpZVelocity (Variables|/Script/Engine.Character|GetCharacterMovement (stale Ability|EventActivateAbility _ashermes_player_character)) (Variables|Default|GetJumpVelocitySave))
  (Ability|EndAbility))

(event Ability|EventActivateAbility
  (Development|PrintString "GA_HighJump")
  (bind _ashermes_player_character (Utilities|Casting|CastToHermesPlayerCharacter (Ability|GetAvatarActorfromActorInfo)))
  (Variables|Default|SetJumpVelocitySave (Variables|/Script/Engine.CharacterMovementComponent|GetJumpZVelocity (Variables|/Script/Engine.Character|GetCharacterMovement _ashermes_player_character)))
  (Variables|/Script/Engine.CharacterMovementComponent|SetJumpZVelocity (Variables|/Script/Engine.Character|GetCharacterMovement _ashermes_player_character) (Variables|Default|GetHighJumpVelocity))
  (Character|Jump _ashermes_player_character)
  (EventDispatchers|AssignLandedDelegate _ashermes_player_character (delegate Custom|LandedDelegate_이벤트)))

(event Ability|EventOnEndAbility
  (params (bWasCancelled :type Boolean)))