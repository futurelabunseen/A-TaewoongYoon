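; Base player character Blueprint that wires up a health bar widget and a deployable glider.
; On BeginPlay it casts its HPBar component's widget to HPBar and sets itself as the target actor.
; Glider input calls the parent handler, then shows the glider and sets the gliding state if the character is falling.
; Switching to walking or flying movement hides the glider and clears gliding.
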(event EventBeginPlay
  (bind _ashpbar (Utilities|Casting|CastToHPBar (UserInterface|GetWidget (Variables|Default|GetHPBar))))
  (Variables|/Game/UI/HPBar.HPBar_C|SetTargetActor _ashpbar self))

(event Collision|EventActorBeginOverlap
  (params (OtherActor :type Actor%20Object%20Reference)))

(event EventTick
  (params (DeltaSeconds :type Float%20%28single-precision%29)))

(event EventGliderInputPressed
  (|CallParentFunction)
  (if (AI|Components|NavMovement|IsFalling (Variables|Character|GetCharacterMovement))
    (CallFunction|EnableGlider)))

(event EventOnMovementModeChanged
  (params (PrevMovementMode :type EMovementMode%20Enum :default "MOVE_None") (NewMovementMode :type EMovementMode%20Enum :default "MOVE_None") (PrevCustomMode :type Byte :default 0) (NewCustomMode :type Byte :default 0))
  (if (or (Utilities|Enum|Equal(Enum) NewMovementMode "MOVE_Walking") (Utilities|Enum|Equal(Enum) NewMovementMode "MOVE_Flying"))
    (CallFunction|DisableGlider)))

(fn ConstructionScript)

(fn EnableGlider
  (Development|SetHiddeninGame (Variables|Default|GetGlider) false false)
  (Class|HermesPlayerCharacter|SetIsGliding true))

(fn DisableGlider
  (Development|SetHiddeninGame (Variables|Default|GetGlider) true false)
  (Class|HermesPlayerCharacter|SetIsGliding false))